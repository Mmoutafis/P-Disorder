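; Wisp-like enemy NPC that damages the player on overlap and shows negative thoughts, counting itself in DisorderGameMode's enemy tally.
; Overlap deals damage on a one-second cooldown and, if the player's Hit flag is set, displays a random taunt every few seconds.
; NegativeThoughtsText builds each taunt from per-letter Niagara systems with swapped textures.
; Low health slows it, disables collision, swaps to death particles, plays a sound, then destroys it.
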(event OnComponentBeginOverlap(Box)
  (params (OverlappedComponent :type Primitive%20Component%20Object%20Reference) (OtherActor :type Actor%20Object%20Reference) (OtherComp :type Primitive%20Component%20Object%20Reference) (OtherBodyIndex :type Integer) (bFromSweep :type Boolean) (SweepResult :type Hit%20Result%20Structure%20%28by%20ref%29))
  (bind _asplayer_character_test (Utilities|Casting|CastToPlayerCharacterTest OtherActor))
  (Variables|Default|SetAs%20Player%20Character%20Test _asplayer_character_test)
  (Utilities|FlowControl|Sequence
    (:then_0
      (Utilities|FlowControl|DoOnce false :!label _label
        (:Completed
          (Game|Damage|ApplyDamage _asplayer_character_test 1e+01 0 0)
          (Development|PrintString "Hit")
          (Utilities|FlowControl|Delay 1.0)
          (goto _label Reset))))
    (:then_1
      (if (Variables|/Game/MichaelM/Blueprints/PlayerCharacterTest.PlayerCharacterTest_C|GetHit? (Variables|Default|GetAs%20Player%20Character%20Test))
        (Utilities|FlowControl|DoOnce false :!label _label_2
          (:Completed
            (CallFunction|NegativeThoughtsText (.OutItem (Utilities|Array|Random (Variables|Default|GetNegative%20Text%20Array))) (Transformation|GetActorLocation (Variables|Default|GetAs%20Player%20Character%20Test)))
            (Utilities|FlowControl|Delay 4.0)
            (goto _label_2 Reset)))))))

(event EventBeginPlay
  (bind _negative_text_array (Variables|Default|GetNegative%20Text%20Array))
  (bind _asdisorder_game_mode (Utilities|Casting|CastToDisorderGameMode (Game|GetGameMode)))
  (Variables|Default|SetAs%20Disorder%20Game%20Mode _asdisorder_game_mode)
  (Default|IncreaseEnemies _asdisorder_game_mode)
  (Utilities|Array|Add _negative_text_array (Variables|Default|GetYou%20should%20Leave!))
  (Utilities|Array|Add _negative_text_array (Variables|Default|GetNobody%20believes%20you!!))
  (Utilities|Array|Add _negative_text_array (Variables|Default|GetAre%20you%20even%20real))
  (Utilities|Array|Add _negative_text_array (Variables|Default|GetParanoid))
  (Utilities|Array|Add _negative_text_array (Variables|Default|GetScared)))

(event Game|Damage|EventAnyDamage
  (params (Damage :type Float%20%28single-precision%29) (DamageType :type Damage%20Type%20Object%20Reference) (InstigatedBy :type Controller%20Object%20Reference) (DamageCauser :type Actor%20Object%20Reference))
  (Variables|Default|SetHealth (- (Variables|Default|GetHealth) Damage))
  (if (< (Variables|Default|GetHealth) 1e+01)
    (Variables|/Script/Engine.CharacterMovementComponent|SetMaxWalkSpeed (Variables|Character|GetCharacterMovement) 5e+01)
    (Collision|SetActorEnableCollision false)
    (Components|Activation|SetActive (Variables|Default|GetParticleSystem1) false false)
    (Components|Activation|SetActive (Variables|Default|GetDeath%20particle) true false)
    (Utilities|FlowControl|Delay 1.0)
    (Utilities|FlowControl|Sequence
      (:then_0
        (Components|Activation|SetActive (Variables|Default|GetDeath%20particle1) false false)
        (Utilities|FlowControl|Delay 3.0)
        (Actor|DestroyActor)
        (Default|DecreaseEnemies (Variables|Default|GetAs%20Disorder%20Game%20Mode)))
      (:then_1
        (Audio|PlaySoundatLocation "/Game/ChristopherR/Audio/SFX/WispDeath.WispDeath" (Transformation|GetActorLocation) "0, 0, 0" 1.0 1.0 0.0 0 0 0)))))

(fn ConstructionScript)

(fn NegativeThoughtsText
  (params (Text :type String) (Location :type Vector))
  (bind _as_player_character_test (Variables|Default|GetAs%20Player%20Character%20Test))
  (bind _mesh (Variables|/Script/Engine.Character|GetMesh _as_player_character_test))
  (bind _returnvalue (Transformation|GetWorldLocation _mesh))
  (for _array_element (Utilities|String|GetCharacterArrayfromString Text)
    (bind _returnvalue_2 (Niagara|SpawnSystematLocation "/Game/MichaelM/Blueprints/TextVisualiser/TextVisualiserNiagaraSystem.TextVisualiserNiagaraSystem" (Math|Vector|MakeVector (+ (.x _returnvalue) -1.5e+02) (+ (.y _returnvalue) 2.5e+02) (+ (.z _returnvalue) 3.5e+02)) (Math|Rotator|MakeRotator (Math|Random|RandomFloatinRange 1.3e+02 1.5e+02) (Math|Random|RandomFloatinRange 1.8e+02 2e+02) (- (.yaw (Transformation|GetWorldRotation (Variables|/Game/MichaelM/Blueprints/PlayerCharacterTest.PlayerCharacterTest_C|GetCamera1 _as_player_character_test))) 9e+01)) "0.200000,0.200000,0.200000"))
    (bind _output_get (LocalVariables|SetTextSystem _returnvalue_2))
    (Transformation|AddLocalOffset _output_get (Math|Vector|MakeVector (LocalVariables|GetTextOffset) 0.0 0.0) false false)
    (LocalVariables|SetTextOffset (+ (LocalVariables|GetTextOffset) 5e+01))
    (switch string _array_element
      (:a
        (Niagara|SetTextureObject (LocalVariables|GetTextSystem) "Texture" "/Game/MichaelM/Blueprints/TextVisualiser/Textures/A.A"))
      (:b
        (Niagara|SetTextureObject (LocalVariables|GetTextSystem) "Texture" "/Game/MichaelM/Blueprints/TextVisualiser/Textures/B.B"))
      (:c
        (Niagara|SetTextureObject (LocalVariables|GetTextSystem) "Texture" "/Game/MichaelM/Blueprints/TextVisualiser/Textures/C.C"))
      (:d
        (Niagara|SetTextureObject (LocalVariables|GetTextSystem) "Texture" "/Game/MichaelM/Blueprints/TextVisualiser/Textures/D.D"))
      (:e
        (Niagara|SetTextureObject (LocalVariables|GetTextSystem) "Texture" "/Game/MichaelM/Blueprints/TextVisualiser/Textures/E.E"))
      (:f
        (Niagara|SetTextureObject (LocalVariables|GetTextSystem) "Texture" "/Game/MichaelM/Blueprints/TextVisualiser/Textures/F.F"))
      (:g
        (Niagara|SetTextureObject (LocalVariables|GetTextSystem) "Texture" "/Game/MichaelM/Blueprints/TextVisualiser/Textures/G.G"))
      (:h
        (Niagara|SetTextureObject (LocalVariables|GetTextSystem) "Texture" "/Game/MichaelM/Blueprints/TextVisualiser/Textures/H.H"))
      (:i
        (Niagara|SetTextureObject (LocalVariables|GetTextSystem) "Texture" "/Game/MichaelM/Blueprints/TextVisualiser/Textures/I.I"))
      (:j
        (Niagara|SetTextureObject (LocalVariables|GetTextSystem) "Texture" "/Game/MichaelM/Blueprints/TextVisualiser/Textures/J.J"))
      (:k
        (Niagara|SetTextureObject (LocalVariables|GetTextSystem) "Texture" "/Game/MichaelM/Blueprints/TextVisualiser/Textures/K.K"))
      (:l
        (Niagara|SetTextureObject (LocalVariables|GetTextSystem) "Texture" "/Game/MichaelM/Blueprints/TextVisualiser/Textures/L.L"))
      (:m
        (Niagara|SetTextureObject (LocalVariables|GetTextSystem) "Texture" "/Game/MichaelM/Blueprints/TextVisualiser/Textures/M.M"))
      (:n
        (Niagara|SetTextureObject (LocalVariables|GetTextSystem) "Texture" "/Game/MichaelM/Blueprints/TextVisualiser/Textures/N.N"))
      (:o
        (Niagara|SetTextureObject (LocalVariables|GetTextSystem) "Texture" "/Game/MichaelM/Blueprints/TextVisualiser/Textures/O.O"))
      (:p
        (Niagara|SetTextureObject (LocalVariables|GetTextSystem) "Texture" "/Game/MichaelM/Blueprints/TextVisualiser/Textures/P.P"))
      (:q
        (Niagara|SetTextureObject (LocalVariables|GetTextSystem) "Texture" "/Game/MichaelM/Blueprints/TextVisualiser/Textures/Q.Q"))
      (:r
        (Niagara|SetTextureObject (LocalVariables|GetTextSystem) "Texture" "/Game/MichaelM/Blueprints/TextVisualiser/Textures/R.R"))
      (:s
        (Niagara|SetTextureObject (LocalVariables|GetTextSystem) "Texture" "/Game/MichaelM/Blueprints/TextVisualiser/Textures/S.S"))
      (:t
        (Niagara|SetTextureObject (LocalVariables|GetTextSystem) "Texture" "/Game/MichaelM/Blueprints/TextVisualiser/Textures/T.T"))
      (:u
        (Niagara|SetTextureObject (LocalVariables|GetTextSystem) "Texture" "/Game/MichaelM/Blueprints/TextVisualiser/Textures/U.U"))
      (:v
        (Niagara|SetTextureObject (LocalVariables|GetTextSystem) "Texture" "/Game/MichaelM/Blueprints/TextVisualiser/Textures/V.V"))
      (:w
        (Niagara|SetTextureObject (LocalVariables|GetTextSystem) "Texture" "/Game/MichaelM/Blueprints/TextVisualiser/Textures/W.W"))
      (:x
        (Niagara|SetTextureObject (LocalVariables|GetTextSystem) "Texture" "/Game/MichaelM/Blueprints/TextVisualiser/Textures/X.X"))
      (:y
        (Niagara|SetTextureObject (LocalVariables|GetTextSystem) "Texture" "/Game/MichaelM/Blueprints/TextVisualiser/Textures/Y.Y"))
      (:z
        (Niagara|SetTextureObject (LocalVariables|GetTextSystem) "Texture" "/Game/MichaelM/Blueprints/TextVisualiser/Textures/Z.Z"))
      (:!
        (Niagara|SetTextureObject (LocalVariables|GetTextSystem) "Texture" "/Game/MichaelM/Blueprints/TextVisualiser/Textures/Exclimation_Mark.Exclimation_Mark"))
      (:?
        (Niagara|SetTextureObject (LocalVariables|GetTextSystem) "Texture" "/Game/MichaelM/Blueprints/TextVisualiser/Textures/Question_MArk.Question_MArk")))))