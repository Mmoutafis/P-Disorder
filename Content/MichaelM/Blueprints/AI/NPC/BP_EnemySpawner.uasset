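; BP_EnemySpawner is a placed spawner that keeps creating BP_Enemy AI in batches at its root location.
; It spawns a first batch on BeginPlay, then caches the DisorderGameMode.
; After each spawn delay, it spawns another batch only while EnemiesAlive is below the game mode's MaxEnemies.
; Otherwise, ShouldSpawn re-checks on the same delay, forming an endless recursive polling loop without Tick or timers.
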(event Custom|Spawn%20Enemy
  (params (PawnClass :type Pawn%20Class%20Reference) (LastIndex :type Integer))
  (bind _as_disorder_game_mode (Variables|Default|GetAs%20Disorder%20Game%20Mode))
  (for _index (range 0 (- LastIndex 1))
    (AI|SpawnAIFromClass PawnClass 0 (Transformation|GetWorldLocation (Variables|Default|GetDefaultSceneRoot)) "0, 0, 0" false 0))
  (Utilities|FlowControl|Delay (Variables|Default|GetSpawn%20Delay))
  (if (< (Variables|/Game/MichaelM/Blueprints/DisorderGameMode.DisorderGameMode_C|GetEnemies%20Alive _as_disorder_game_mode) (Variables|/Game/MichaelM/Blueprints/DisorderGameMode.DisorderGameMode_C|GetMax%20Enemies _as_disorder_game_mode))
    (CallFunction|SpawnEnemy "/Game/MichaelM/Blueprints/AI/NPC/BP_Enemy.BP_Enemy_C" (Variables|Default|Getnumber%20of%20enemies))
    (else
      (CallFunction|ShouldSpawn))))

(event Custom|Should%20Spawn
  (bind _as_disorder_game_mode (Variables|Default|GetAs%20Disorder%20Game%20Mode))
  (Utilities|FlowControl|Delay (Variables|Default|GetSpawn%20Delay))
  (if (< (Variables|/Game/MichaelM/Blueprints/DisorderGameMode.DisorderGameMode_C|GetEnemies%20Alive _as_disorder_game_mode) (Variables|/Game/MichaelM/Blueprints/DisorderGameMode.DisorderGameMode_C|GetMax%20Enemies _as_disorder_game_mode))
    (CallFunction|SpawnEnemy "/Game/MichaelM/Blueprints/AI/NPC/BP_Enemy.BP_Enemy_C" (Variables|Default|Getnumber%20of%20enemies))
    (else
      (CallFunction|ShouldSpawn))))

(event EventBeginPlay
  (Utilities|FlowControl|Sequence
    (:then_0
      (CallFunction|SpawnEnemy "/Game/MichaelM/Blueprints/AI/NPC/BP_Enemy.BP_Enemy_C" (Variables|Default|Getnumber%20of%20enemies)))
    (:then_1
      (bind _asdisorder_game_mode (Utilities|Casting|CastToDisorderGameMode (Game|GetGameMode)))
      (Variables|Default|SetAs%20Disorder%20Game%20Mode _asdisorder_game_mode))))

(fn ConstructionScript)