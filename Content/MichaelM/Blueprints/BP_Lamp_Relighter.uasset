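; BP_Lamp_Relighter is a candle interaction point where pressing E while nearby sets Health to 100 and prints "healed".
; Box overlap by PlayerCharacterTest toggles the EToRelight prompt and NearCandle, with a lighter sound through a DoOnce reset on exit.
; Health is a local copy of the player's value taken at BeginPlay, and nothing writes it back.
; A second volume, Box1, hides StaticMesh1 while the player overlaps it.
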(event OnComponentBeginOverlap(Box)
  (params (OverlappedComponent :type Primitive%20Component%20Object%20Reference) (OtherActor :type Actor%20Object%20Reference) (OtherComp :type Primitive%20Component%20Object%20Reference) (OtherBodyIndex :type Integer) (bFromSweep :type Boolean) (SweepResult :type Hit%20Result%20Structure%20%28by%20ref%29))
  (Utilities|Casting|CastToPlayerCharacterTest OtherActor)
  (Development|SetHiddeninGame (Variables|Default|GetE%20to%20relight) false false)
  (Variables|Default|SetNear%20Candle? true)
  (Utilities|FlowControl|DoOnce false
    (:Completed
      (Audio|PlaySound2D "/Game/ChristopherR/Audio/SFX/524097__spacejoe__lighter-3.524097__spacejoe__lighter-3" 1.0 1.0 0.0 0 0))))

(event OnComponentEndOverlap(Box)
  (params (OverlappedComponent :type Primitive%20Component%20Object%20Reference) (OtherActor :type Actor%20Object%20Reference) (OtherComp :type Primitive%20Component%20Object%20Reference) (OtherBodyIndex :type Integer))
  (Utilities|Casting|CastToPlayerCharacterTest OtherActor)
  (Development|SetHiddeninGame (Variables|Default|GetE%20to%20relight) true false)
  (Variables|Default|SetNear%20Candle? false)
  (Utilities|FlowControl|DoOnce false) ; enters at Reset
)

(event OnComponentBeginOverlap(Box1)
  (params (OverlappedComponent :type Primitive%20Component%20Object%20Reference) (OtherActor :type Actor%20Object%20Reference) (OtherComp :type Primitive%20Component%20Object%20Reference) (OtherBodyIndex :type Integer) (bFromSweep :type Boolean) (SweepResult :type Hit%20Result%20Structure%20%28by%20ref%29))
  (Utilities|Casting|CastToPlayerCharacterTest OtherActor)
  (Rendering|SetVisibility (Variables|Default|GetStaticMesh1) false false))

(event OnComponentEndOverlap(Box1)
  (params (OverlappedComponent :type Primitive%20Component%20Object%20Reference) (OtherActor :type Actor%20Object%20Reference) (OtherComp :type Primitive%20Component%20Object%20Reference) (OtherBodyIndex :type Integer))
  (Utilities|Casting|CastToPlayerCharacterTest OtherActor)
  (Rendering|SetVisibility (Variables|Default|GetStaticMesh1) true false))

(event EventBeginPlay
  (bind _asplayer_character_test (Utilities|Casting|CastToPlayerCharacterTest (Game|GetPlayerCharacter 0)))
  (Variables|Default|SetHealth (Variables|/Game/MichaelM/Blueprints/PlayerCharacterTest.PlayerCharacterTest_C|GetHealth _asplayer_character_test)))

(event EventTick
  (params (DeltaSeconds :type Float%20%28single-precision%29)))

(event Input|KeyboardEvents|E
  (params (Key :type Key%20Structure :default "None"))
  (:Pressed
    (if (Variables|Default|GetNear%20Candle?)
      (Variables|Default|SetHealth 1e+02)
      (Development|PrintString "healed"))))

(fn ConstructionScript)