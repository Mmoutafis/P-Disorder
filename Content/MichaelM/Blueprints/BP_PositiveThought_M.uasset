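; Collectible positive thought pickup that reacts when the player character overlaps its box collider.
; On pickup it plays a sound, disables collision, calls DestroyPath on DisorderGameMode and animates the sphere's dynamic material Appearance while toggling its own and the player's particles.
; It then increments the game mode's PositiveThoughtCount, drives Emissive Mult in the player material parameter collection through one of two count-selected timelines, and destroys itself after a delay.
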(event OnComponentBeginOverlap(BoxCollider)
  (params (OverlappedComponent :type Primitive%20Component%20Object%20Reference) (OtherActor :type Actor%20Object%20Reference) (OtherComp :type Primitive%20Component%20Object%20Reference) (OtherBodyIndex :type Integer) (bFromSweep :type Boolean) (SweepResult :type Hit%20Result%20Structure%20%28by%20ref%29))
  (bind _asplayer_character_test (Utilities|Casting|CastToPlayerCharacterTest OtherActor))
  (Variables|Default|SetParticle%20System (Variables|/Game/MichaelM/Blueprints/PlayerCharacterTest.PlayerCharacterTest_C|GetParticleSystem _asplayer_character_test))
  (Utilities|FlowControl|Sequence
    (:then_0
      (Variables|Default|SetDestroyed true)
      (Default|DestroyPath (Variables|Default|GetAs%20Top%20Down%20Game%20Mode%201))
      (Collision|SetActorEnableCollision false)
      (bind _returnvalue (Rendering|Material|CreateDynamicMaterialInstance (Variables|Default|GetSphere) 0 "/Game/MichaelM/Materials/M_Positive_Thoughts_Main_Inst.M_Positive_Thoughts_Main_Inst" "None" :!class /Script/Engine.PrimitiveComponent))
      (bind _newtrack_0 (Timeline|Timeline_0 Play)
        (:Update
          (Rendering|Material|SetScalarParameterValue _returnvalue "Appearance" _newtrack_0 :!class /Script/Engine.MaterialInstanceDynamic)
          (Components|Activation|SetActive (Variables|Default|GetParticleSystem) false false)
          (Utilities|FlowControl|Delay 0.2)
          (Utilities|FlowControl|DoOnce false :!label _label
            (:Completed
              (Components|Activation|SetActive (Variables|Default|GetParticle%20System) true false)
              (Utilities|FlowControl|Delay 1.0)
              (Components|Activation|SetActive (Variables|Default|GetParticle%20System) false false)
              (goto _label Reset))))
        (:Finished
          (bind _asdisorder_game_mode (Utilities|Casting|CastToDisorderGameMode (Game|GetGameMode)))
          (bind _output_get (Variables|Default|SetPositive%20Thought%20Count (Variables|/Game/MichaelM/Blueprints/DisorderGameMode.DisorderGameMode_C|GetPositive%20Thought%20Count _asdisorder_game_mode)))
          (bind _output_get_2 (Variables|/Game/MichaelM/Blueprints/DisorderGameMode.DisorderGameMode_C|SetPositive%20Thought%20Count _asdisorder_game_mode (+ _output_get 1.0)))
          (Development|PrintString (Utilities|String|ToString(Float) _output_get_2))
          (bind _returnvalue_2 (Rendering|Material|GetScalarParameterValue "/Game/MichaelM/Materials/Player_collection.Player_collection" "Emissive Mult" :!class /Script/Engine.KismetMaterialLibrary))
          (Variables|Default|SetEmmisive%20Mult _returnvalue_2)
          (if (>= (Variables|Default|GetPositive%20Thought%20Count) 1.0)
            (bind _newtrack_0_2 (Timeline|Timeline_2 Play)
              (:Update
                (Rendering|Material|SetScalarParameterValue "/Game/MichaelM/Materials/Player_collection.Player_collection" "Emissive Mult" _newtrack_0_2 :!class /Script/Engine.KismetMaterialLibrary)
                (Utilities|FlowControl|Delay 3.0)
                (Actor|DestroyActor)))
            (else
              (bind _newtrack_0_3 (Timeline|Timeline_1 Play)
                (:Update
                  (Rendering|Material|SetScalarParameterValue "/Game/MichaelM/Materials/Player_collection.Player_collection" "Emissive Mult" _newtrack_0_3 :!class /Script/Engine.KismetMaterialLibrary)
                  (Utilities|FlowControl|Delay 3.0)
                  (Actor|DestroyActor))))))))
    (:then_1
      (Audio|PlaySound2D "/Game/ChristopherR/Audio/SFX/561188__toasthatter__soul-pickup.561188__toasthatter__soul-pickup" 1.0 1.0 0.0 0 0))))

(event EventBeginPlay
  (Variables|Default|SetLocation (Transformation|GetActorLocation))
  (bind _asdisorder_game_mode (Utilities|Casting|CastToDisorderGameMode (Game|GetGameMode)))
  (Variables|Default|SetAs%20Top%20Down%20Game%20Mode%201 _asdisorder_game_mode))

(fn ConstructionScript)

(fn SelectPositiveThought)