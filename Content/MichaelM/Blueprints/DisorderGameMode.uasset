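; DisorderGameMode is a game mode that manages a guide path from the player to the nearest positive thought.
; Tick recomputes the navmesh path and feeds it to BP_PathTracerMichael, which events show or hide.
; DestroyPath hides the tracer and pauses redrawing for six seconds via a DoOnce-gated Delay.
; It also starts ambient sound, fades it after that delay if PositiveThoughtCount is positive, and tracks living enemies.
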(event Custom|Illuminate_Path
  ;[1 1 1] Path System
  (if (not (Variables|Default|GetDestroyed?))
    (Rendering|SetActorHiddenInGame (Variables|Default|GetLine%20tracer) false)))

(event Custom|Fade%20Out%20path
  ;[1 1 1] Path System
  (if (not (Variables|Default|GetDestroyed?))
    (Rendering|SetActorHiddenInGame (Variables|Default|GetLine%20tracer) true)))

(event Custom|Increase%20enemies
  ;[1 1 1] Path System
  (Math|Integer|IncrementInt (Variables|Default|GetEnemies%20Alive)))

(event Custom|Decrease%20Enemies
  ;[1 1 1] Path System
  (Math|Integer|DecrementInt (Variables|Default|GetEnemies%20Alive)))

(event EventTick
  (params (DeltaSeconds :type Float%20%28single-precision%29))
  ;[1 1 1] Path System
  (if (Variables|Default|GetDestroyed?)
    (Utilities|FlowControl|DoOnce false :!label _label
      (:Completed
        (Utilities|FlowControl|Delay 6.0)
        (CallFunction|DrawPath)
        (Variables|Default|SetDestroyed? false)
        (if (> (Variables|Default|GetPositive%20Thought%20Count) 0.0)
          (Utilities|FlowControl|DoOnce false
            (:Completed
              (Audio|Components|Audio|FadeOut (stale EventBeginPlay _returnvalue) 0.0 0.0 "Linear" :!class /Script/Engine.AudioComponent))))))
    (else
      (CallFunction|DrawPath)
      (goto _label Reset))))

(event EventBeginPlay
  ;[1 1 1] Path System
  (bind _outactors (Actor|GetAllActorsOfClass "/Game/PathTracer/Blueprints/BP_PathTracerMichael.BP_PathTracerMichael_C"))
  (Variables|Default|SetLine%20tracer (Utilities|Array|Get(acopy) _outactors))
  (bind _returnvalue (Audio|CreateSound2D (Variables|Default|GetAmbient%20Sound) 1.0 1.0 0.0 0))
  (Audio|Components|Audio|Play _returnvalue 0.0)
  (Rendering|SetActorHiddenInGame (Variables|Default|GetLine%20tracer) true))

(fn ConstructionScript)

(fn DrawPath
  (bind _line_tracer (Variables|Default|GetLine%20tracer))
  (bind _outactors (Actor|GetAllActorsOfClass "/Game/MichaelM/Blueprints/BP_PositiveThought_M.BP_PositiveThought_M_C"))
  (bind _output_get (Variables|Default|SetClosest%20Positive%20Thought (.ReturnValue (Actor|FindNearestActor (Transformation|GetActorLocation (Game|GetPlayerCharacter 0)) _outactors))))
  (bind _returnvalue (Class|NavigationSystemV1|FindPathtoLocationSynchronously (Transformation|GetActorLocation (Game|GetPlayerCharacter 0)) (Transformation|GetActorLocation _output_get) 0 0))
  (bind _output_get_2 (Variables|Default|SetPath%20Points (Variables|/Script/NavigationSystem.NavigationPath|GetPathPoints _returnvalue)))
  (bind _asbp_path_tracer_michael (Utilities|Casting|CastToBP_PathTracerMichael _line_tracer))
  (Utilities|IsValid _line_tracer
    (:Is%20Valid
      (Default|DrawPath _asbp_path_tracer_michael _output_get_2))))

(fn DestroyPath
  (Rendering|SetActorHiddenInGame (Variables|Default|GetLine%20tracer) true)
  (Variables|Default|SetDestroyed? true))