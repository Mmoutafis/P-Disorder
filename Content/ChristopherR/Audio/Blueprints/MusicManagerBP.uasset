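; MusicManagerBP is a music manager that switches between tracks in a level.
; On BeginPlay it creates a 2D sound for each TrackList entry, starts all of them silent at once, then raises the chosen opening track to MusicVolume.
; ChangeMusicTo mutes the current track and unmutes the requested index, so switches are instant volume swaps between already-playing tracks, and prints the new track's name.
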(event Custom|ChangeMusicTo
  (params (IndexOfSongToPlay :type Integer))
  (bind _musicreferences (Variables|Default|GetMusicReferences))
  (bind _output (Utilities|Array|Get(acopy) _musicreferences IndexOfSongToPlay))
  (Utilities|IsValid (Variables|Default|GetCurrentMusicRef)
    (:Is%20Valid
      (Audio|Components|Audio|SetVolumeMultiplier (Variables|Default|GetCurrentMusicRef) 0.0 :!class /Script/Engine.AudioComponent))
    (:Is%20Not%20Valid
      _))
  (Audio|Components|Audio|SetVolumeMultiplier _output (Variables|Default|GetMusicVolume) :!class /Script/Engine.AudioComponent)
  (bind _output_get (Variables|Default|SetCurrentMusicRef _output))
  (Development|PrintString (Utilities|String|Append "Music playing" (Utilities|GetDisplayName _output_get))))

(event EventBeginPlay
  (bind _musicreferences (Variables|Default|GetMusicReferences))
  (bind _indexofsongtoplayonlevelbegin (Variables|Default|GetIndexOfSongToPlayOnLevelBegin))
  (bind _output (Utilities|Array|Get(acopy) _musicreferences _indexofsongtoplayonlevelbegin))
  (for _array_element (Variables|Default|GetTrackList)
    (bind _returnvalue (Audio|CreateSound2D _array_element 1.0 1.0 0.0 0))
    (Utilities|IsValid _returnvalue
      (:Is%20Valid
        (Utilities|Array|Add (Variables|Default|GetMusicReferences) _returnvalue)
        (Audio|Components|Audio|SetVolumeMultiplier _returnvalue 0.0 :!class /Script/Engine.AudioComponent)
        (Audio|Components|Audio|Play _returnvalue 0.0))))
  (Audio|Components|Audio|SetVolumeMultiplier _output (Variables|Default|GetMusicVolume) :!class /Script/Engine.AudioComponent)
  (Variables|Default|SetCurrentMusicRef _output))

(fn ConstructionScript)