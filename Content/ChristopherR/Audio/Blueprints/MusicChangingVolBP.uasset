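; MusicChangingVolBP is a trigger volume that switches the game's music when the player enters it.
; On BeginPlay it finds the level's MusicManagerBP and caches the first one found.
; When the player pawn first overlaps the Box, it passes MusicToPlayOnOverlap to the manager's ChangeMusicTo.
; A DoOnce with no reset makes each volume fire only once.
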(event OnComponentBeginOverlap(Box)
  (params (OverlappedComponent :type Primitive%20Component%20Object%20Reference) (OtherActor :type Actor%20Object%20Reference) (OtherComp :type Primitive%20Component%20Object%20Reference) (OtherBodyIndex :type Integer) (bFromSweep :type Boolean) (SweepResult :type Hit%20Result%20Structure%20%28by%20ref%29))
  (if (== OtherActor (Game|Player|GetPlayerPawn 0))
    (Utilities|FlowControl|DoOnce false
      (:Completed
        (Default|ChangeMusicto (Variables|Default|GetMusic%20Manager%20Ref) (Variables|Default|GetMusic%20To%20Play%20On%20Overlap))))))

(event EventBeginPlay
  (bind _outactors (Actor|GetAllActorsOfClass "/Game/ChristopherR/Audio/Blueprints/MusicManagerBP.MusicManagerBP_C"))
  (Variables|Default|SetMusic%20Manager%20Ref (Utilities|Array|Get(acopy) _outactors)))

(fn ConstructionScript)